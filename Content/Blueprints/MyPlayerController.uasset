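; Player controller that sets up local two-player movement from a single set of input bindings.
; On BeginPlay it spawns a second controller and a Player2 pawn at a fixed location, then has that controller possess the pawn.
; It handles both players' movement axes itself, moving its own pawn and Player2 along each one's control rotation forward and right vectors.
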(event EventTick
  (params (DeltaSeconds :type Float%20%28single-precision%29)))

(event EventBeginPlay
  (bind _returnvalue (Math|Transform|MakeTransform "0.000000,50.000000,300.000000"))
  ;[1 1 1] Spawn n set controller then actor
  (bind _returnvalue_2 (Game|SpawnActorfromClass "/Game/Blueprints/MyPlayerController_2.MyPlayerController_2_C" _returnvalue "Undefined" 0 0))
  (Variables|Default|Setcontroller2 _returnvalue_2)
  (bind _returnvalue_3 (Game|SpawnActorfromClass "/Game/Blueprints/Player2.Player2_C" _returnvalue "Undefined" 0 0))
  (Variables|Default|Setplayer2 _returnvalue_3)
  ;[1 1 1] Possess Target
  (Pawn|Possess (Variables|Default|Getcontroller2) (Variables|Default|Getplayer2)))

(event Input|AxisEvents|InputAxisMoveForward2
  (params (AxisValue :type Float%20%28single-precision%29))
  (bind _player2 (Variables|Default|Getplayer2))
  ;[1 1 1] Movement Player 2
  (Pawn|Input|AddMovementInput _player2 (Math|Vector|GetForwardVector (Pawn|GetControlRotation _player2 :!class /Script/Engine.Pawn)) AxisValue false))

(event Input|AxisEvents|InputAxisMoveSideways2
  (params (AxisValue :type Float%20%28single-precision%29))
  (bind _player2 (Variables|Default|Getplayer2))
  ;[1 1 1] Movement Player 2
  (Pawn|Input|AddMovementInput _player2 (Math|Vector|GetRightVector (Pawn|GetControlRotation _player2 :!class /Script/Engine.Pawn)) AxisValue false))

(event Input|AxisEvents|InputAxisMoveForward
  (params (AxisValue :type Float%20%28single-precision%29))
  (bind _returnvalue (Pawn|GetControlledPawn))
  ;[1 1 1] Movement Player1
  (Pawn|Input|AddMovementInput _returnvalue (Math|Vector|GetForwardVector (Pawn|GetControlRotation _returnvalue :!class /Script/Engine.Pawn)) AxisValue false))

(event Input|AxisEvents|InputAxisMoveSideways
  (params (AxisValue :type Float%20%28single-precision%29))
  (bind _returnvalue (Pawn|GetControlledPawn))
  ;[1 1 1] Movement Player1
  (Pawn|Input|AddMovementInput _returnvalue (Math|Vector|GetRightVector (Pawn|GetControlRotation _returnvalue :!class /Script/Engine.Pawn)) AxisValue false))

(fn ConstructionScript)